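; BP_GameMode is a game mode that splits joining players into two teams.
; On PostLogin it casts the player to BP_MultiPlayerController, compares team sizes, then sets the team ID and adds the controller to that team's array.
; Team 1 receives the player only when it is smaller, so ties go to Team 2.
; Logout only prints a debug string and leaves the team arrays unchanged.
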(event EventBeginPlay)

(event EventTick
  (params (DeltaSeconds :type Float%20%28single-precision%29)))

(event EventPostLogin
  (params (NewPlayer :type Player%20Controller%20Object%20Reference))
  (bind _asbp_multi_player_controller (Utilities|Casting|CastToBP_MultiPlayerController NewPlayer))
  (if (< (Utilities|Array|Length (Variables|Default|GetTeam1)) (Utilities|Array|Length (Variables|Default|GetTeam2)))
    (Default|SetTeamId _asbp_multi_player_controller 1)
    (Utilities|Array|Add (Variables|Default|GetTeam1) _asbp_multi_player_controller)
    (else
      (Default|SetTeamId _asbp_multi_player_controller 2)
      (Utilities|Array|Add (Variables|Default|GetTeam2) _asbp_multi_player_controller))))

(event EventOnLogout
  (params (ExitingController :type Controller%20Object%20Reference))
  (Development|PrintString "logout"))

(fn ConstructionScript)