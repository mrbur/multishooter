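; BP_Projectile is a multiplayer projectile that damages BP_MultiplayerPawn actors it overlaps, ignoring its owner.
; The server moves it forward each tick by setting its location without sweep, and a BeginPlay timer destroys it after TTL.
; On a server-side sphere overlap, it applies damage, destroys itself, then calls a multicast hit effect, which receives a zero location rather than the impact point.
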(event OnComponentBeginOverlap(Sphere1)
  (params (OverlappedComponent :type Primitive%20Component%20Object%20Reference) (OtherActor :type Actor%20Object%20Reference) (OtherComp :type Primitive%20Component%20Object%20Reference) (OtherBodyIndex :type Integer) (bFromSweep :type Boolean) (SweepResult :type Hit%20Result%20Structure%20%28by%20ref%29))
  (if (Networking|IsServer)
    (CallFunction|ServerColission OtherActor "0, 0, 0")))

(event Custom|EndLife
  (CallFunction|ServerEndlife))

(event Custom|server_endlife
  (Actor|DestroyActor))

(event Custom|server_move
  (params (deltatime :type Float%20%28single-precision%29))
  (Transformation|SetActorLocation (+ (Transformation|GetActorLocation) (* (Transformation|GetActorForwardVector) (* deltatime (Variables|Default|GetSpeed)))) false false))

(event Custom|server_colission
  (params (other%20actor :type Actor%20Object%20Reference) (location :type Vector))
  (if (!= other%20actor (Components|GetOwner))
    (bind _asbp_multiplayer_pawn (Utilities|Casting|CastToBP_MultiplayerPawn other%20actor))
    (Default|CustomEvent0 _asbp_multiplayer_pawn)
    (Default|ServerTakedamage _asbp_multiplayer_pawn (Variables|Default|GetDamage))
    (CallFunction|ServerEndlife)
    (CallFunction|MulticastHiteffect location)))

(event Custom|SpawnHitEffect
  (params (hitLocation :type Vector))
  (Effects|SpawnEmitteratLocation 0 hitLocation))

(event Custom|Multicast_hiteffect
  (params (location :type Vector))
  (CallFunction|SpawnHitEffect location))

(event EventBeginPlay
  (Utilities|Time|SetTimerbyEvent (delegate Custom|EndLife) (Variables|Default|GetTTL)))

(event Collision|EventActorBeginOverlap
  (params (OtherActor :type Actor%20Object%20Reference)))

(event EventTick
  (params (DeltaSeconds :type Float%20%28single-precision%29))
  (if (Networking|IsServer)
    (CallFunction|ServerMove DeltaSeconds)))

(fn ConstructionScript)